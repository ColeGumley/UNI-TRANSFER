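; Projectile actor that flies in a straight line and destroys enemies on contact, despite the enemy-projectile name.
; Tick moves it along local X by Speed each frame, without delta-time scaling, and feeds a two-second Delay that destroys it as a lifetime limit.
; A hitbox overlap casts to BP_enemy1, then BP_enemy2, destroying both the matched enemy and the projectile; other actors are ignored.
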(event `self.ReceiveTick`
  (params (DeltaSeconds :type "Float (single-precision)"))
  ; shooting
  (`self.K2_AddActorLocalOffset` (`KismetMathLibrary.MakeVector` (`self.speed`)))
  (`KismetSystemLibrary.Delay` 2.0)
  (`self.K2_DestroyActor`))

(event `self.projectile_hitbox.OnComponentBeginOverlap`
  (params (OverlappedComponent :type "PrimitiveComponent Object Reference") (OtherActor :type "Actor Object Reference") (OtherComp :type "PrimitiveComponent Object Reference") (OtherBodyIndex :type Integer) (bFromSweep :type Boolean) (SweepResult :type "HitResult Structure (by ref)"))
  ; enemy collision
  (bind _asbp_enemy_1 (cast `/Game/Blueprints/Enemies/BP_enemy1` OtherActor)
    (:`then`
      (`self.K2_DestroyActor` _asbp_enemy_1)
      (`self.K2_DestroyActor`))
    (:`CastFailed`
      (bind _asbp_enemy_2 (cast `/Game/Blueprints/Enemies/BP_enemy2` OtherActor))
      (`self.K2_DestroyActor` _asbp_enemy_2)
      (`self.K2_DestroyActor`))))

(fn `UserConstructionScript`)