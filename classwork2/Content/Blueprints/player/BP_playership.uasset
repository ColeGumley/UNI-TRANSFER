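; Player ship for a shooter, with movement input, mouse-based rotation, HUD and music.
; Keys select pistol, shotgun, uzi or flamethrower modes, which spawn the same projectile class, mostly alternating left and right cannons via FlipFlop.
; Shots drain energy, regenerated through a delay on Tick, and firing stops when depleted.
; Enemy contact destroys the enemy and deals damage with red flash, grunt and brief invulnerability; death returns to the main menu.
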(event `self.ReceiveBeginPlay`
  ; inputs
  (`self.Player inputs`)
  (`GameplayStatics.PlaySound2D` "/Game/Sounds/572947__jibey__rock-music.572947__jibey__rock-music" 1.0 1.0 0.0 null null)
  (bind _returnvalue (`|CreateWidget` "/Game/UI/BP_HUD.BP_HUD_C"))
  (`UserWidget.AddToViewport` _returnvalue 0))

(event `EnhancedInput|/Game/core/IA_movement`
  (params (ActionValue :type "Vector2D Structure") (ElapsedSeconds :type "Float (double-precision)") (TriggeredSeconds :type "Float (double-precision)") (InputAction :type "InputAction Object Reference" :default "/Game/core/IA_movement.IA_movement"))
  ; Movement
  (:`Triggered`
    (`self.AddMovementInput` (1.0 0.0 0.0) ActionValue_X)
    (`self.AddMovementInput` (0.0 1.0 0.0) ActionValue_Y)))

(event `Key|Escape`
  (params (Key :type "Key Structure"))
  ; Close to menu
  (:`Pressed`
    (`GameplayStatics.OpenLevel` "L_MainMenu")))

(event `self.ReceiveTick`
  (params (DeltaSeconds :type "Float (single-precision)"))
  (bind (_locationx _locationy) (`WidgetLayoutLibrary.GetMousePositionScaledByDPI` null))
  ; Movement
  ;; Rotation
  (`|ExecutionSequence`
    (:`then_0`
      (`self.K2_SetActorRotation` (`GameplayStatics.GetPlayerPawn` 0) (`KismetMathLibrary.FindLookAtRotation` (`KismetMathLibrary.MakeVector` _locationx _locationy) (`KismetMathLibrary.MakeVector` (.x (`.WorldDirection` (`PlayerController.DeprojectMousePositionToWorld` (`GameplayStatics.GetPlayerController` 0)))) (.y (`.WorldDirection` (`PlayerController.DeprojectMousePositionToWorld` (`GameplayStatics.GetPlayerController` 0)))))) false))
    (:`then_1`
      (`WidgetLayoutLibrary.GetMousePositionOnViewport`))
    (:`then_2`
      ; energy regen
      (`KismetSystemLibrary.Delay` 0.25)
      (bind _result (`/Engine/EditorBlueprintResources/StandardMacros.IncrementFloat` (`self.CurrentEnergy`))
        (:`  `
          (if (>= _result 1.0)
            (set `self.No energy` false)))))))

(event `EnhancedInput|/Game/core/IA_combat`
  (params (ActionValue :type Boolean) (ElapsedSeconds :type "Float (double-precision)") (TriggeredSeconds :type "Float (double-precision)") (InputAction :type "InputAction Object Reference" :default "/Game/core/IA_combat.IA_combat"))
  ; combat
  (:`Triggered`
    (if (== (`self.Firing_mode`) 1)
      (if (not (`self.No energy`))
        (`KismetSystemLibrary.Delay` 0.25)
        (`/Engine/EditorBlueprintResources/StandardMacros.FlipFlop`
          (:`A`
            (`self.single shot_R`)
            (`self.EnergyDrainPistol`))
          (:`B`
            (`self.single shot_L`)
            (`self.EnergyDrainPistol`))))
      (elif (== (`self.Firing_mode`) 2)
        (if (not (`self.No energy`))
          (`KismetSystemLibrary.Delay` 0.3)
          (`/Engine/EditorBlueprintResources/StandardMacros.FlipFlop`
            (:`A`
              (`self.Shotgun_L`)
              (`self.EnergyDrainShotgun`))
            (:`B`
              (`self.Shotgun_R`)
              (`self.EnergyDrainShotgun`))))
        (elif (== (`self.Firing_mode`) 3)
          (if (not (`self.No energy`))
            (`KismetSystemLibrary.Delay` 0.1)
            (`/Engine/EditorBlueprintResources/StandardMacros.FlipFlop`
              (:`A`
                (`self.Uzi_R`)
                (`self.EnergyDrainUzi`))
              (:`B`
                (`self.Uzi_L`)
                (`self.EnergyDrainUzi`))))
          (elif (== (`self.Firing_mode`) 4)
            (if (not (`self.No energy`))
              (`KismetSystemLibrary.Delay` 0.01)
              (`self.Flamethrower_C`)
              (`self.EnergyDrainFlamethrower`))))))))

(event `Key|One`
  (params (Key :type "Key Structure"))
  ; combat
  ;; switch firing modes
  (:`Pressed`
    (`GameplayStatics.PlaySoundAtLocation` "/Game/Sounds/sound_effects/669488__geoff-bremner-audio__clink-chunk-mechanical.669488__geoff-bremner-audio__clink-chunk-mechanical" (`self.K2_GetActorLocation`) (struct) 1.0 1.0 0.0 null null null null)
    (set `self.Firing_mode` 1)))

(event `Key|Two`
  (params (Key :type "Key Structure"))
  ; combat
  ;; switch firing modes
  (:`Pressed`
    (`GameplayStatics.PlaySoundAtLocation` "/Game/Sounds/sound_effects/669488__geoff-bremner-audio__clink-chunk-mechanical.669488__geoff-bremner-audio__clink-chunk-mechanical" (`self.K2_GetActorLocation`) (struct) 1.0 1.0 0.0 null null null null)
    (set `self.Firing_mode` 2)))

(event `Key|Three`
  (params (Key :type "Key Structure"))
  ; combat
  ;; switch firing modes
  (:`Pressed`
    (`GameplayStatics.PlaySoundAtLocation` "/Game/Sounds/sound_effects/669488__geoff-bremner-audio__clink-chunk-mechanical.669488__geoff-bremner-audio__clink-chunk-mechanical" (`self.K2_GetActorLocation`) (struct) 1.0 1.0 0.0 null null null null)
    (set `self.Firing_mode` 3)))

(event `Key|Four`
  (params (Key :type "Key Structure"))
  ; combat
  ;; switch firing modes
  (:`Pressed`
    (`GameplayStatics.PlaySoundAtLocation` "/Game/Sounds/sound_effects/669488__geoff-bremner-audio__clink-chunk-mechanical.669488__geoff-bremner-audio__clink-chunk-mechanical" (`self.K2_GetActorLocation`) (struct) 1.0 1.0 0.0 null null null null)
    (set `self.Firing_mode` 4)))

(event `self.Box collision.OnComponentBeginOverlap`
  (params (OverlappedComponent :type "PrimitiveComponent Object Reference") (OtherActor :type "Actor Object Reference") (OtherComp :type "PrimitiveComponent Object Reference") (OtherBodyIndex :type Integer) (bFromSweep :type Boolean) (SweepResult :type "HitResult Structure (by ref)"))
  ; collisions & Health
  (bind _asbp_enemy_1 (cast `/Game/Blueprints/Enemies/BP_enemy1` OtherActor)
    (:`then`
      (`GameplayStatics.ApplyDamage` self 20.0 null _asbp_enemy_1)
      (`self.K2_DestroyActor` _asbp_enemy_1))
    (:`CastFailed`
      (bind _asbp_enemy_2 (cast `/Game/Blueprints/Enemies/BP_enemy2` OtherActor))
      (`GameplayStatics.ApplyDamage` self 10.0 null _asbp_enemy_2)
      (`self.K2_DestroyActor` _asbp_enemy_2))))

(event `self.ReceiveAnyDamage`
  (params (Damage :type "Float (single-precision)") (DamageType :type "DamageType Object Reference") (InstigatedBy :type "Controller Object Reference") (DamageCauser :type "Actor Object Reference"))
  ; collisions & Health
  (`|ExecutionSequence`
    (:`then_0`
      (if (not (`self.IFrames`))
        (bind _returnvalue (`KismetMaterialLibrary.CreateDynamicMaterialInstance` "/Game/Blueprints/player/M_playership.M_playership"))
        (bind _output_get (set `self.damage player` _returnvalue))
        (`MaterialInstanceDynamic.SetVectorParameterValue` _returnvalue "damage player" (struct :`R` 1.0 :`B` 0.030547 :`A` 1.0))
        (`MaterialInstanceDynamic.SetVectorParameterValue` _output_get "damage player" (struct :`R` 1.0 :`B` 0.030547 :`A` 1.0))
        (`PrimitiveComponent.SetMaterial` (`self.ship`) 0 (`self.damage player`))
        (`KismetSystemLibrary.Delay` 0.2)
        (bind _output_get_2 (set `self.damage player` (`self.damage player`)))
        (`MaterialInstanceDynamic.SetVectorParameterValue` :`self` _output_get_2 :`ParameterName` "damage player")
        (`/Engine/EditorBlueprintResources/StandardMacros.FlipFlop`
          (:`A`
            (`GameplayStatics.PlaySoundAtLocation` "/Game/Sounds/sound_effects/547198__mrfossy__voice_adultmale_paingrunts_15.547198__mrfossy__voice_adultmale_paingrunts_15" (`self.K2_GetActorLocation`) (struct) 1.0 1.0 0.0 null null null null))
          (:`B`
            (`GameplayStatics.PlaySoundAtLocation` "/Game/Sounds/sound_effects/795466__aulix24__grunt-1.795466__aulix24__grunt-1" (`self.K2_GetActorLocation`) (struct) 1.0 1.0 0.0 null null null null)))))
    (:`then_1`
      (if (not (`self.IFrames`))
        (bind _output_get_3 (set `self.Current health` (- (`self.Current health`) Damage)))
        (if (`self.is dead`)
          (`GameplayStatics.OpenLevel` "L_MainMenu")
          (else
            (set `self.IFrames` true)
            (`KismetSystemLibrary.Delay` 0.5)
            (set `self.IFrames` false)
            (set `self.is dead` (<= (`KismetMathLibrary.FClamp` _output_get_3 0.0 (`self.Max health`)) 0.0))))))))

(fn `EnergyDrainFlamethrower`
  (bind _output_get (set `self.CurrentEnergy` (- (`self.CurrentEnergy`) 2.0)))
  (if (<= (`KismetMathLibrary.FClamp` _output_get 0.0 (`self.MaxEnergy`)) 0.0)
    (set `self.No energy` true)))

(fn `EnergyDrainPistol`
  (bind _output_get (set `self.CurrentEnergy` (- (`self.CurrentEnergy`) 1.0)))
  (if (<= (`KismetMathLibrary.FClamp` _output_get 0.0 (`self.MaxEnergy`)) 0.0)
    (set `self.No energy` true)))

(fn `EnergyDrainShotgun`
  (bind _output_get (set `self.CurrentEnergy` (- (`self.CurrentEnergy`) 6.0)))
  (if (<= (`KismetMathLibrary.FClamp` _output_get 0.0 (`self.MaxEnergy`)) 0.0)
    (set `self.No energy` true)))

(fn `EnergyDrainUzi`
  (bind _output_get (set `self.CurrentEnergy` (- (`self.CurrentEnergy`) 2.0)))
  (if (<= (`KismetMathLibrary.FClamp` _output_get 0.0 (`self.MaxEnergy`)) 0.0)
    (set `self.No energy` true)))

(fn `Flamethrower_C`
  (`|SpawnActorFromClass` "/Game/Blueprints/projectiles/BP_player-projectile.BP_player-projectile_C" (`KismetMathLibrary.MakeTransform` (`SceneComponent.K2_GetComponentLocation` (`self.Main_C_Cannon`)) (`self.K2_GetActorRotation`)) "Undefined" "MultiplyWithRoot" null null))

(fn `Player inputs`
  (bind _returnvalue (pcsubsystem `EnhancedInputLocalPlayerSubsystem` (`GameplayStatics.GetPlayerController` 0)))
  (`EnhancedInputSubsystemInterface.AddMappingContext` _returnvalue "/Game/core/IMC_Movement.IMC_Movement" 0 (struct))
  (`EnhancedInputSubsystemInterface.AddMappingContext` _returnvalue "/Game/core/IMC_combat.IMC_combat" 0 (struct)))

(fn `Shotgun_L`
  (bind (_returnvalue_roll _returnvalue_pitch _returnvalue_yaw) (`KismetMathLibrary.BreakRotator` (`self.K2_GetActorRotation`)))
  (bind (_returnvalue_roll_2 _returnvalue_pitch_2 _returnvalue_yaw_2) (`KismetMathLibrary.BreakRotator` (`self.K2_GetActorRotation`)))
  (`|SpawnActorFromClass` "/Game/Blueprints/projectiles/BP_player-projectile.BP_player-projectile_C" (`KismetMathLibrary.MakeTransform` (`SceneComponent.K2_GetComponentLocation` (`self.Main_L_cannon`)) (`KismetMathLibrary.MakeRotator` _returnvalue_roll_2 _returnvalue_pitch_2 (+ _returnvalue_yaw_2 5.0))) "Undefined" "MultiplyWithRoot" null null)
  (`GameplayStatics.PlaySound2D` "/Game/Sounds/sound_effects/734060__dthetech__dd-shotgun-2c.734060__dthetech__dd-shotgun-2c" 1.0 1.0 0.0 null null)
  (`|SpawnActorFromClass` "/Game/Blueprints/projectiles/BP_player-projectile.BP_player-projectile_C" (`KismetMathLibrary.MakeTransform` (`SceneComponent.K2_GetComponentLocation` (`self.L_cannon2`)) (`KismetMathLibrary.MakeRotator` _returnvalue_roll _returnvalue_pitch (+ _returnvalue_yaw -5.0))) "Undefined" "MultiplyWithRoot" null null)
  (`|SpawnActorFromClass` "/Game/Blueprints/projectiles/BP_player-projectile.BP_player-projectile_C" (`KismetMathLibrary.MakeTransform` (`SceneComponent.K2_GetComponentLocation` (`self.L_cannon3`)) (`self.K2_GetActorRotation`)) "Undefined" "MultiplyWithRoot" null null))

(fn `Shotgun_R`
  (bind (_returnvalue_roll _returnvalue_pitch _returnvalue_yaw) (`KismetMathLibrary.BreakRotator` (`self.K2_GetActorRotation`)))
  (bind (_returnvalue_roll_2 _returnvalue_pitch_2 _returnvalue_yaw_2) (`KismetMathLibrary.BreakRotator` (`self.K2_GetActorRotation`)))
  (`|SpawnActorFromClass` "/Game/Blueprints/projectiles/BP_player-projectile.BP_player-projectile_C" (`KismetMathLibrary.MakeTransform` (`SceneComponent.K2_GetComponentLocation` (`self.Main_R_cannon`)) (`KismetMathLibrary.MakeRotator` _returnvalue_roll _returnvalue_pitch (+ _returnvalue_yaw 5.0))) "Undefined" "MultiplyWithRoot" null null)
  (`GameplayStatics.PlaySound2D` "/Game/Sounds/sound_effects/734060__dthetech__dd-shotgun-2c.734060__dthetech__dd-shotgun-2c" 1.0 1.0 0.0 null null)
  (`|SpawnActorFromClass` "/Game/Blueprints/projectiles/BP_player-projectile.BP_player-projectile_C" (`KismetMathLibrary.MakeTransform` (`SceneComponent.K2_GetComponentLocation` (`self.R_cannon2`)) (`KismetMathLibrary.MakeRotator` _returnvalue_roll_2 _returnvalue_pitch_2 (+ _returnvalue_yaw_2 -5.0))) "Undefined" "MultiplyWithRoot" null null)
  (`|SpawnActorFromClass` "/Game/Blueprints/projectiles/BP_player-projectile.BP_player-projectile_C" (`KismetMathLibrary.MakeTransform` (`SceneComponent.K2_GetComponentLocation` (`self.R_cannon3`)) (`self.K2_GetActorRotation`)) "Undefined" "MultiplyWithRoot" null null))

(fn `single shot_L`
  (`|SpawnActorFromClass` "/Game/Blueprints/projectiles/BP_player-projectile.BP_player-projectile_C" (`KismetMathLibrary.MakeTransform` (`SceneComponent.K2_GetComponentLocation` (`self.Main_L_cannon`)) (`self.K2_GetActorRotation`)) "Undefined" "MultiplyWithRoot" null null)
  (`GameplayStatics.PlaySound2D` "/Game/Sounds/sound_effects/734097__modusmogulus__gunshot-forest-2m-harsh.734097__modusmogulus__gunshot-forest-2m-harsh" 1.0 1.0 0.0 null null))

(fn `single shot_R`
  (`|SpawnActorFromClass` "/Game/Blueprints/projectiles/BP_player-projectile.BP_player-projectile_C" (`KismetMathLibrary.MakeTransform` (`SceneComponent.K2_GetComponentLocation` (`self.Main_R_cannon`)) (`self.K2_GetActorRotation`)) "Undefined" "MultiplyWithRoot" null null)
  (`GameplayStatics.PlaySound2D` "/Game/Sounds/sound_effects/734097__modusmogulus__gunshot-forest-2m-harsh.734097__modusmogulus__gunshot-forest-2m-harsh" 1.0 1.0 0.0 null null))

(fn `UserConstructionScript`)

(fn `Uzi_L`
  (`|SpawnActorFromClass` "/Game/Blueprints/projectiles/BP_player-projectile.BP_player-projectile_C" (`KismetMathLibrary.MakeTransform` (`SceneComponent.K2_GetComponentLocation` (`self.Main_L_cannon`)) (`self.K2_GetActorRotation`)) "Undefined" "MultiplyWithRoot" null null)
  (`GameplayStatics.PlaySound2D` "/Game/Sounds/sound_effects/734097__modusmogulus__gunshot-forest-2m-harsh.734097__modusmogulus__gunshot-forest-2m-harsh" 1.0 1.0 0.0 null null))

(fn `Uzi_R`
  (`|SpawnActorFromClass` "/Game/Blueprints/projectiles/BP_player-projectile.BP_player-projectile_C" (`KismetMathLibrary.MakeTransform` (`SceneComponent.K2_GetComponentLocation` (`self.Main_R_cannon`)) (`self.K2_GetActorRotation`)) "Undefined" "MultiplyWithRoot" null null)
  (`GameplayStatics.PlaySound2D` "/Game/Sounds/sound_effects/734097__modusmogulus__gunshot-forest-2m-harsh.734097__modusmogulus__gunshot-forest-2m-harsh" 1.0 1.0 0.0 null null))