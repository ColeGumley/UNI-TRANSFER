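; BP_plane is a player-controlled plane driven by Enhanced Input, with a spinning propeller.
; BeginPlay adds the IMC_Movement mapping context to the first player's input subsystem.
; IA_movement's X axis feeds movement along the actor's forward vector, while Y both rolls the plane and moves it along the fixed world Y axis.
; Tick rolls the Propella component by a constant amount each frame, independent of delta time.
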(event `self.ReceiveTick`
  (params (DeltaSeconds :type "Float (single-precision)"))
  (`SceneComponent.K2_AddLocalRotation` (`self.Propella`) (`KismetMathLibrary.MakeRotator` 8.0) false false))

(event `self.ReceiveBeginPlay`
  (`EnhancedInputSubsystemInterface.AddMappingContext` (pcsubsystem `EnhancedInputLocalPlayerSubsystem` (`GameplayStatics.GetPlayerController` 0)) "/Game/core/IMC_Movement.IMC_Movement" 0 (struct)))

(event `EnhancedInput|/Game/core/IA_movement`
  (params (ActionValue :type "Vector2D Structure") (ElapsedSeconds :type "Float (double-precision)") (TriggeredSeconds :type "Float (double-precision)") (InputAction :type "InputAction Object Reference" :default "/Game/core/IA_movement.IA_movement"))
  (:`Triggered`
    (`self.AddMovementInput` (`self.GetActorForwardVector`) ActionValue_X)
    (`self.K2_AddActorLocalRotation` (`KismetMathLibrary.MakeRotator` ActionValue_Y))
    (`self.AddMovementInput` (0.0 1.0 0.0) ActionValue_Y)))

(fn `UserConstructionScript`)