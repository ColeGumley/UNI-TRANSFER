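; BP_enemy2 is an enemy that homes in on the player, takes damage and awards score when killed in GM_Endless.
; Each tick it sweeps forward by a fixed, frame-rate-dependent step and turns to face the player pawn.
; Damage plays a hit sound, briefly flashes the Plane red through a new dynamic material instance, and reduces health.
; At zero health it adds score, spawns a Niagara death burst and destroys itself.
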(event `self.ReceiveTick`
  (params (DeltaSeconds :type "Float (single-precision)"))
  (`self.K2_AddActorLocalOffset` (5.0 0.0 0.0) true)
  (`self.K2_SetActorRotation` (`KismetMathLibrary.FindLookAtRotation` (`self.K2_GetActorLocation`) (`self.K2_GetActorLocation` (`GameplayStatics.GetPlayerPawn` 0)))))

(event `self.ReceiveDestroyed`)

(event `self.ReceiveAnyDamage`
  (params (Damage :type "Float (single-precision)") (DamageType :type "DamageType Object Reference") (InstigatedBy :type "Controller Object Reference") (DamageCauser :type "Actor Object Reference"))
  (`|ExecutionSequence`
    (:`then_0`
      (`GameplayStatics.PlaySoundAtLocation` "/Game/Sounds/sound_effects/547042__cogfirestudios__hit-impact-sword-3.547042__cogfirestudios__hit-impact-sword-3" (`self.K2_GetActorLocation`) (struct) 1.0 1.0 0.0 null null null null))
    (:`then_1`
      (`self.hit reg`)
      (bind _output_get (set `self.current health` (- (`self.current health`) Damage)))
      (set `self.is dead` (<= (`KismetMathLibrary.FClamp` _output_get 0.0 (`self.Max health`)) 0.0))
      (if (`self.is dead`)
        (bind _asgm_endless (cast `/Game/core/GM_Endless` (`GameplayStatics.GetGameMode`)))
        (`/Game/core/GM_Endless.Add Score` _asgm_endless)
        (`NiagaraFunctionLibrary.SpawnSystemAtLocation` "/Game/VFX/NS_DeathBurst.NS_DeathBurst" (`self.K2_GetActorLocation`))
        (`self.K2_DestroyActor`)))))

(event `hit reg`
  (bind _returnvalue (`KismetMaterialLibrary.CreateDynamicMaterialInstance` "/Game/Materials/M_Metal_silver.M_Metal_silver"))
  (bind _output_get (set `self.matflash` _returnvalue))
  (`MaterialInstanceDynamic.SetVectorParameterValue` _returnvalue "DMGFlash" (struct :`R` 1.0 :`B` 0.030547 :`A` 1.0))
  (`MaterialInstanceDynamic.SetVectorParameterValue` _output_get "DMGFlash" (struct :`R` 1.0 :`B` 0.030547 :`A` 1.0))
  (`PrimitiveComponent.SetMaterial` (`self.Plane`) 0 (`self.matflash`))
  (`KismetSystemLibrary.Delay` 0.2)
  (bind _output_get_2 (set `self.matflash` (`self.matflash`)))
  (`MaterialInstanceDynamic.SetVectorParameterValue` :`self` _output_get_2 :`ParameterName` "DMGFlash"))

(fn `UserConstructionScript`)