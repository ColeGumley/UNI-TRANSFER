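; BP_Spawner is an enemy spawner actor that continuously produces two enemy types, BP_enemy1 and BP_enemy2.
; On BeginPlay it starts two looping half-second timers by function name, one for each enemy type.
; Each timer function spawns its enemy at the spawner's location with a random offset along world Y, spreading spawns across a wide line.
; It has no spawn cap or stop condition.
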(event `self.ReceiveBeginPlay`
  (`|ExecutionSequence`
    (:`then_0`
      (`KismetSystemLibrary.K2_SetTimer` null "SpawnEnemy1" 0.5 true))
    (:`then_1`
      (`KismetSystemLibrary.K2_SetTimer` null "Spawn enemy 2" 0.5 true))))

(fn `Spawn enemy 2`
  (bind (_returnvalue_x _returnvalue_y _returnvalue_z) (`KismetMathLibrary.BreakVector` (`self.K2_GetActorLocation`)))
  (`|SpawnActorFromClass` "/Game/Blueprints/Enemies/BP_enemy2.BP_enemy2_C" (`KismetMathLibrary.MakeTransform` (`KismetMathLibrary.MakeVector` _returnvalue_x (+ _returnvalue_y (`KismetMathLibrary.RandomFloatInRange` -11000.0 11000.0)) _returnvalue_z)) "Undefined" "MultiplyWithRoot" null null))

(fn `SpawnEnemy1`
  (bind (_returnvalue_x _returnvalue_y _returnvalue_z) (`KismetMathLibrary.BreakVector` (`self.K2_GetActorLocation`)))
  (`|SpawnActorFromClass` "/Game/Blueprints/Enemies/BP_enemy1.BP_enemy1_C" (`KismetMathLibrary.MakeTransform` (`KismetMathLibrary.MakeVector` _returnvalue_x (+ _returnvalue_y (`KismetMathLibrary.RandomFloatInRange` -11000.0 11000.0)) _returnvalue_z)) "Undefined" "MultiplyWithRoot" null null))

(fn `UserConstructionScript`)