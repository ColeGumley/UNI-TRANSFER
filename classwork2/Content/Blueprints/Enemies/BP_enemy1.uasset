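; BP_enemy1 is a simple enemy actor that charges in a straight line and can drop pickups when destroyed.
; On BeginPlay it rotates to face the player pawn once, then moves forward a fixed local offset every tick, without sweep or delta-time scaling.
; On Destroyed it spawns a Niagara death burst, then has a half chance to drop either a health or energy restore pickup, with equal odds.
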(event `self.ReceiveDestroyed`
  ; Death & Powerup drops
  (`NiagaraFunctionLibrary.SpawnSystemAtLocation` "/Game/VFX/NS_DeathBurst.NS_DeathBurst" (`self.K2_GetActorLocation`))
  (if (>= (`KismetMathLibrary.RandomInteger` 10) 5)
    (if (>= (`KismetMathLibrary.RandomInteger` 10) 5)
      (`|SpawnActorFromClass` "/Game/Blueprints/pickups/BP_Health_restore.BP_Health_restore_C" (`KismetMathLibrary.MakeTransform` (`self.K2_GetActorLocation`)) "Undefined" "MultiplyWithRoot" null null)
      (else
        (`|SpawnActorFromClass` "/Game/Blueprints/pickups/BP_Energy_restore.BP_Energy_restore_C" (`KismetMathLibrary.MakeTransform` (`self.K2_GetActorLocation`)) "Undefined" "MultiplyWithRoot" null null)))))

(event `self.ReceiveTick`
  (params (DeltaSeconds :type "Float (single-precision)"))
  ; movement
  (`self.K2_AddActorLocalOffset` (5.0 0.0 0.0)))

(event `self.ReceiveBeginPlay`
  ; movement
  (`self.K2_SetActorRotation` (`KismetMathLibrary.FindLookAtRotation` (`self.K2_GetActorLocation`) (`self.K2_GetActorLocation` (`GameplayStatics.GetPlayerPawn` 0)))))

(fn `UserConstructionScript`)